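; BP_Meteor_Character is a character Blueprint that tracks movement speed and input state.
; Each Tick it stores forward speed as the dot product of velocity and the capsule's forward vector.
; The Attack and Left input actions set held-state flags on press and clear them on release.
; A matching right-speed calculation exists but is not connected to execution, and nothing in this graph reads the stored values.
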(event `self.ReceiveTick`
  (params (DeltaSeconds :type "Float (single-precision)"))
  (`|ExecutionSequence`
    (:`then_0`
      (set `self.move_fwd_speed` (`KismetMathLibrary.Dot_VectorVector` (`self.GetVelocity`) (`SceneComponent.GetForwardVector` (`self.CapsuleComponent`)))))))

(event `InputAction|Attack`
  (params (Key :type "Key Structure" :default "AnyKey"))
  (:`Pressed`
    (set `self.IsAttackPress` true))
  (:`Released`
    (set `self.IsAttackPress` false)))

(event `InputAction|Left`
  (params (Key :type "Key Structure" :default "AnyKey"))
  (:`Pressed`
    (set `self.IsLeftKeyDown` true))
  (:`Released`
    (set `self.IsLeftKeyDown` false)))

(fn `UserConstructionScript`)